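; Actor component that tracks the player character's health and stamina, including their maximums.
; On BeginPlay it casts its owner to BP_ThirdPersonCharacter and caches it for HUD access.
; Each change function writes directly to that character's HUD bars and text, with increases to current values capped at the maximum.
; DecHealth returns true at zero or below, while DecStam returns false there; neither clamps at zero.
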(event `AssignStats`
  (bind _asbp_third_person_character (cast `/Game/ThirdPerson/Blueprints/BP_ThirdPersonCharacter` (`self.GetOwner`)))
  (set `self.PlayerCharBP` _asbp_third_person_character))

(event `self.ReceiveBeginPlay`
  (`self.AssignStats`))

(fn `DecHealth`
  (params (Damage :type "Float (double-precision)"))
  (returns (IsPlayerDead :type Boolean))
  (bind _hudwidget (`/Game/ThirdPerson/Blueprints/BP_ThirdPersonCharacter.HUDWidget` (`self.PlayerCharBP`)))
  ;[0.05127 0.05127 0.05127] Decrease
  (bind _output_get (set `self.CurrentHP` (- (`self.CurrentHP`) Damage)))
  (`ProgressBar.SetPercent` (`/Game/UI/WB_HUD.Health` _hudwidget) (/ _output_get (`self.MaxHP`)))
  (`TextBlock.SetText` (`/Game/UI/WB_HUD.healthText` _hudwidget) (`KismetTextLibrary.Conv_DoubleToText` (`self.CurrentHP`) "HalfToEven"))
  (if (<= (`self.CurrentHP`) 0.0)
    (return true)
    (else
      (return false))))

(fn `DecStam`
  (params (DepleteAmount :type "Float (double-precision)"))
  (returns (StamGone :type Boolean))
  (bind _hudwidget (`/Game/ThirdPerson/Blueprints/BP_ThirdPersonCharacter.HUDWidget` (`self.PlayerCharBP`)))
  (set `self.CurrentStam` (- (`self.CurrentStam`) DepleteAmount))
  (`ProgressBar.SetPercent` (`/Game/UI/WB_HUD.Stamina` _hudwidget) (/ (`self.CurrentStam`) (`self.MaxStam`)))
  (`TextBlock.SetText` (`/Game/UI/WB_HUD.StamText` _hudwidget) (`KismetTextLibrary.Conv_DoubleToText` (`self.CurrentStam`) "HalfToEven"))
  (if (<= (`self.CurrentStam`) 0.0)
    (return false)
    (else
      (return true))))

(fn `Inc Max Health`
  (params (MaxHPup :type "Float (double-precision)"))
  (bind _hudwidget (`/Game/ThirdPerson/Blueprints/BP_ThirdPersonCharacter.HUDWidget` (`self.PlayerCharBP`)))
  (set `self.MaxHP` (+ (`self.MaxHP`) MaxHPup))
  (`ProgressBar.SetPercent` (`/Game/UI/WB_HUD.Health` _hudwidget) (/ (`self.CurrentHP`) (`self.MaxHP`)))
  (`TextBlock.SetText` (`/Game/UI/WB_HUD.healthText` _hudwidget) (`KismetTextLibrary.Conv_DoubleToText` (`self.CurrentHP`) "HalfToEven")))

(fn `Inc Max Stam`
  (params (AdditionalStam :type "Float (double-precision)"))
  (bind _hudwidget (`/Game/ThirdPerson/Blueprints/BP_ThirdPersonCharacter.HUDWidget` (`self.PlayerCharBP`)))
  (set `self.MaxStam` (+ (`self.MaxStam`) AdditionalStam))
  (`ProgressBar.SetPercent` (`/Game/UI/WB_HUD.Stamina` _hudwidget) (/ (`self.CurrentStam`) (`self.MaxStam`)))
  (`TextBlock.SetText` (`/Game/UI/WB_HUD.StamText` _hudwidget) (`KismetTextLibrary.Conv_DoubleToText` (`self.CurrentStam`) "HalfToEven")))

(fn `IncHealth`
  (params (addedHealth :type "Float (double-precision)"))
  (bind _hudwidget (`/Game/ThirdPerson/Blueprints/BP_ThirdPersonCharacter.HUDWidget` (`self.PlayerCharBP`)))
  (set `self.CurrentHP` (+ addedHealth (`self.CurrentHP`)))
  (if (> (`self.CurrentHP`) (`self.MaxHP`))
    (set `self.CurrentHP` (`self.MaxHP`)))
  (`ProgressBar.SetPercent` (`/Game/UI/WB_HUD.Health` _hudwidget) (/ (`self.CurrentHP`) (`self.MaxHP`)))
  (`TextBlock.SetText` (`/Game/UI/WB_HUD.healthText` _hudwidget) (`KismetTextLibrary.Conv_DoubleToText` (`self.CurrentHP`) "HalfToEven")))

(fn `IncStam`
  (params (AddedStam :type "Float (double-precision)"))
  (bind _hudwidget (`/Game/ThirdPerson/Blueprints/BP_ThirdPersonCharacter.HUDWidget` (`self.PlayerCharBP`)))
  (set `self.CurrentStam` (+ (`self.CurrentStam`) AddedStam))
  (if (> (`self.CurrentStam`) (`self.MaxStam`))
    (set `self.CurrentStam` (`self.MaxStam`)))
  (`ProgressBar.SetPercent` (`/Game/UI/WB_HUD.Stamina` _hudwidget) (/ (`self.CurrentStam`) (`self.MaxStam`)))
  (`TextBlock.SetText` (`/Game/UI/WB_HUD.StamText` _hudwidget) (`KismetTextLibrary.Conv_DoubleToText` (`self.CurrentStam`) "HalfToEven")))